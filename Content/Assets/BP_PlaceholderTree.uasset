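; BP_PlaceholderTree is a placeholder tree actor that prototypes a cut interaction.
; Overlap begin and end on its Capsule set and clear a CuttingPosition flag, printing the value, without checking which actor overlaps.
; The Cut input action prints "Cut" while the flag is set, with no actual cutting logic or input-enabling in these graphs.
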(event `self.Capsule.OnComponentBeginOverlap`
  (params (OverlappedComponent :type "PrimitiveComponent Object Reference") (OtherActor :type "Actor Object Reference") (OtherComp :type "PrimitiveComponent Object Reference") (OtherBodyIndex :type Integer) (bFromSweep :type Boolean) (SweepResult :type "HitResult Structure (by ref)"))
  (bind _output_get (set `self.cuttingPosition?` true))
  (`KismetSystemLibrary.PrintString` (`KismetStringLibrary.Conv_BoolToString` _output_get)))

(event `InputAction|Cut`
  (params (Key :type "Key Structure"))
  (:`Pressed`
    (if (`self.cuttingPosition?`)
      (`KismetSystemLibrary.PrintString` "Cut"))))

(event `self.Capsule.OnComponentEndOverlap`
  (params (OverlappedComponent :type "PrimitiveComponent Object Reference") (OtherActor :type "Actor Object Reference") (OtherComp :type "PrimitiveComponent Object Reference") (OtherBodyIndex :type Integer))
  (bind _output_get (set `self.cuttingPosition?` false))
  (`KismetSystemLibrary.PrintString` (`KismetStringLibrary.Conv_BoolToString` _output_get)))

(fn `UserConstructionScript`)
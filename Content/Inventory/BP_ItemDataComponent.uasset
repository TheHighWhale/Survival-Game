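; BP_ItemDataComponent is an item pickup component that stores an ItemID row handle and a Quantity.
; It turns on replication for its owning actor at BeginPlay.
; Interactwith passes the row name and quantity to the player's InventorySystem, then destroys the owner on an always-true branch, without checking the add result.
; LookAt is a stub that returns an empty string.
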(event `self.ReceiveBeginPlay`
  (`Actor.SetReplicates` (`self.GetOwner`) true))

(event `/Game/Inventory/BPI_InteractInterface.InteractWith`
  (params (PlayerCharacter :type "/Game/FirstPerson/Blueprints/BP_FirstPersonCharacter Object Reference"))
  (bind _inventory_system (`/Game/FirstPerson/Blueprints/BP_FirstPersonCharacter.Inventory_System` PlayerCharacter))
  (bind (_itemid_datatable _itemid_rowname) (break `DataTableRowHandle` (`self.ItemID`)))
  (`/Engine/EditorBlueprintResources/StandardMacros.IsValid` _inventory_system
    (:`Is Valid`
      (`/Game/Inventory/BP_InventorySystem.AddToInventory` _inventory_system _itemid_rowname (`self.Quantity`))
      (if true
        (`Actor.K2_DestroyActor` (`self.GetOwner`))))))

(fn `LookAt`
  (returns (Message :type Text))
  (return ""))
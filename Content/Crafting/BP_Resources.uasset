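; BP_Resources detects what the player is looking at, for interaction in the crafting system.
; Every Tick it sphere-traces from the camera along its forward vector up to InteractionRange, ignoring its owner.
; A newly hit actor is cached as LookAtActor and its LookAtMessage result is printed; a miss clears the cache.
; Mine is an empty stub.
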(event `self.ReceiveTick`
  (params (DeltaSeconds :type "Float (single-precision)"))
  (`self.InteractionTrace`))

(fn `InteractionTrace`
  (bind _returnvalue (`GameplayStatics.GetPlayerCameraManager` 0))
  (bind _returnvalue_2 (`Actor.K2_GetActorLocation` _returnvalue))
  (bind (_outhit _returnvalue_3) (`KismetSystemLibrary.SphereTraceSingle` _returnvalue_2 (+ _returnvalue_2 (* (`Actor.GetActorForwardVector` _returnvalue) (`self.InteractionRange`))) 0.0 "TraceTypeQuery3" false (`|MakeArray` (`self.GetOwner`))))
  (if _returnvalue_3
    (bind (_bblockinghit _binitialoverlap _time _distance _location _impactpoint _normal _impactnormal _physmat _hitactor) (`GameplayStatics.BreakHitResult` _outhit))
    (if (!= _hitactor (`self.LookAtActor`))
      (bind _output_get (set `self.LookAtActor` _hitactor))
      (bind _message (message `/Game/Inventory/BPI_InteractInterface.LookAt` _output_get))
      (`KismetSystemLibrary.PrintString` (`KismetTextLibrary.Conv_TextToString` _message)))
    (else
      (set `self.LookAtActor` null))))

(fn `Mine`)
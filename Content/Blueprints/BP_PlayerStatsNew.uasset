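; Player stats Blueprint that tracks health, stamina, XP and level and pushes changes to the player's HUD.
; Increase functions cap health and stamina at their maximums, while decrease functions return whether the value is depleted.
; Reaching max XP triggers a level-up that resets XP and raises the threshold.
; As wired, IncreaseHealth updates its bar only when capping, and IncreaseMaxStamina zeroes stamina instead of adding the increment.
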(fn `Decrease Health`
  (params (Damage :type "Float (double-precision)"))
  (returns (`IsPlayerDead?` :type Boolean))
  (if (not (<= (`self.currentHealth`) 0.0))
    (bind _output_get (set `self.currentHealth` (- (`self.currentHealth`) Damage)))
    (`ProgressBar.SetPercent` (`/Game/UI/WBP_HUD.HealthBar` (`/Game/FirstPerson/Blueprints/BP_FirstPersonCharacter.playerHUD` (`self.Player`))) (/ _output_get (`self.maxHealth`)))
    (if (<= (`self.currentHealth`) 0.0)
      _
      (else
        (return false))))
  (return true))

(fn `Decrease Stamina`
  (params (`Stamina Depleted` :type "Float (double-precision)"))
  (returns (NoStaminaLeft :type Boolean))
  (if (not (<= (`self.currentStamina`) 0.0))
    (bind _output_get (set `self.currentStamina` (- (`self.currentStamina`) `Stamina Depleted`)))
    (`ProgressBar.SetPercent` (`/Game/UI/WBP_HUD.StaminaBar` (`/Game/FirstPerson/Blueprints/BP_FirstPersonCharacter.playerHUD` (`self.Player`))) (/ _output_get (`self.maxStamina`)))
    (if (<= (`self.currentStamina`) 0.0)
      _
      (else
        (return false))))
  (return true))

(fn `Increase Health`
  (params (`Health Added` :type "Float (double-precision)"))
  (set `self.currentHealth` (+ `Health Added` (`self.currentHealth`)))
  (if (> (`self.currentHealth`) (`self.maxHealth`))
    (bind _output_get (set `self.currentHealth` (`self.maxHealth`)))
    (`ProgressBar.SetPercent` (`/Game/UI/WBP_HUD.HealthBar` (`/Game/FirstPerson/Blueprints/BP_FirstPersonCharacter.playerHUD` (`self.Player`))) (/ _output_get (`self.maxHealth`)))))

(fn `Increase Level`
  (set `self.level` (+ (`self.level`) 1))
  (set `self.maxXp` (+ (`self.maxXp`) 10.0))
  (set `self.currentXP` 0.0)
  (`TextBlock.SetText` (`/Game/UI/WBP_HUD.LevelText` (`/Game/FirstPerson/Blueprints/BP_FirstPersonCharacter.playerHUD` (`self.Player`))) (`KismetTextLibrary.Conv_IntToText` (`self.level`))))

(fn `Increase Max Health`
  (params (`Health Increase Increment` :type "Float (double-precision)"))
  (bind _output_get (set `self.maxHealth` (+ (`self.maxHealth`) `Health Increase Increment`)))
  (bind _output_get_2 (set `self.currentHealth` _output_get))
  (`ProgressBar.SetPercent` (`/Game/UI/WBP_HUD.HealthBar` (`/Game/FirstPerson/Blueprints/BP_FirstPersonCharacter.playerHUD` (`self.Player`))) (/ _output_get_2 (`self.maxHealth`))))

(fn `Increase Max Stamina`
  (params (`Stamina Increase Increment` :type "Float (double-precision)"))
  (bind _output_get (set `self.maxStamina` 0.0))
  (bind _output_get_2 (set `self.currentStamina` _output_get))
  (`ProgressBar.SetPercent` (`/Game/UI/WBP_HUD.StaminaBar` (`/Game/FirstPerson/Blueprints/BP_FirstPersonCharacter.playerHUD` (`self.Player`))) (/ _output_get_2 (`self.maxStamina`))))

(fn `Increase Stamina`
  (params (`Stamina Added` :type "Float (double-precision)"))
  (set `self.currentStamina` (+ (`self.currentStamina`) `Stamina Added`))
  (if (> (`self.currentStamina`) (`self.maxStamina`))
    (bind _output_get (set `self.currentStamina` (`self.maxStamina`))))
  (`ProgressBar.SetPercent` (`/Game/UI/WBP_HUD.StaminaBar` (`/Game/FirstPerson/Blueprints/BP_FirstPersonCharacter.playerHUD` (`self.Player`))) (/ _output_get (`self.maxStamina`))))

(fn `Increase XP`
  (params (`XP Gained` :type "Float (double-precision)"))
  (set `self.currentXP` (+ (`self.currentXP`) `XP Gained`))
  (if (>= (`self.currentXP`) (`self.maxXp`))
    (`self.Increase Level`))
  (`ProgressBar.SetPercent` (`/Game/UI/WBP_HUD.XPBar` (`/Game/FirstPerson/Blueprints/BP_FirstPersonCharacter.playerHUD` (`self.Player`))) (/ (`self.currentXP`) (`self.maxXp`)))
  (`TextBlock.SetText` (`/Game/UI/WBP_HUD.XPText` (`/Game/FirstPerson/Blueprints/BP_FirstPersonCharacter.playerHUD` (`self.Player`))) (`|FormatText` "{currentXP} / {maxXP}" (`self.currentXP`) (`self.maxXp`))))
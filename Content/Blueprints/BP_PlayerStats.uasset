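; Player stats component on BP_ThirdPersonCharacter that tracks health, stamina, XP and level.
; After a one-tick delay on BeginPlay it caches the owning character, and its functions write changes straight to that character's HUD widget.
; Decrease functions return whether the stat is depleted, and reaching max XP triggers a level-up with sounds, reset XP and a higher threshold.
; IncreaseMaxStamina zeroes max stamina, leaving its addition unwired.
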(event `self.ReceiveBeginPlay`
  (bind _currentxp (`self.currentXP`))
  (bind _maxxp (`self.maxXP`))
  (`KismetSystemLibrary.DelayUntilNextTick`)
  (bind _asbp_third_person_character (cast `/Game/ThirdPerson/Blueprints/BP_ThirdPersonCharacter` (`self.GetOwner`)))
  (set `self.Player Character BP` _asbp_third_person_character)
  (`ProgressBar.SetPercent` (`/Game/UI/WBP_HUD.StaminaBar` (`/Game/ThirdPerson/Blueprints/BP_ThirdPersonCharacter.HUD Widget` (`self.Player Character BP`))) (/ (`self.currentStamina`) (`self.maxStamina`)))
  (`ProgressBar.SetPercent` (`/Game/UI/WBP_HUD.HealthBar` (`/Game/ThirdPerson/Blueprints/BP_ThirdPersonCharacter.HUD Widget` (`self.Player Character BP`))) (/ (`self.currentHealth`) (`self.maxHealth`)))
  (`ProgressBar.SetPercent` (`/Game/UI/WBP_HUD.XPBar` (`/Game/ThirdPerson/Blueprints/BP_ThirdPersonCharacter.HUD Widget` (`self.Player Character BP`))) (/ _currentxp _maxxp))
  (`TextBlock.SetText` (`/Game/UI/WBP_HUD.XPText` (`/Game/ThirdPerson/Blueprints/BP_ThirdPersonCharacter.HUD Widget` (`self.Player Character BP`))) (`|FormatText` "{currentXP} / {maxXP}" _currentxp _maxxp))
  (`TextBlock.SetText` (`/Game/UI/WBP_HUD.LevelText` (`/Game/ThirdPerson/Blueprints/BP_ThirdPersonCharacter.HUD Widget` (`self.Player Character BP`))) (`KismetTextLibrary.Conv_IntToText` (`self.level`))))

(fn `Decrease Health`
  (params (Damage :type "Float (double-precision)"))
  (returns (`IsPlayerDead?` :type Boolean))
  (if (not (<= (`self.currentHealth`) 0.0))
    (bind _output_get (set `self.currentHealth` (- (`self.currentHealth`) Damage)))
    (`ProgressBar.SetPercent` (`/Game/UI/WBP_HUD.HealthBar` (`/Game/ThirdPerson/Blueprints/BP_ThirdPersonCharacter.HUD Widget` (`self.Player Character BP`))) (/ _output_get (`self.maxHealth`)))
    (if (<= (`self.currentHealth`) 0.0)
      _
      (else
        (return false))))
  (return true))

(fn `Decrease Stamina`
  (params (StaminaDepleted :type "Float (double-precision)"))
  (returns (NoStaminaLeft :type Boolean))
  (if (not (<= (`self.currentStamina`) 0.0))
    (bind _output_get (set `self.currentStamina` (- (`self.currentStamina`) StaminaDepleted)))
    (`ProgressBar.SetPercent` (`/Game/UI/WBP_HUD.StaminaBar` (`/Game/ThirdPerson/Blueprints/BP_ThirdPersonCharacter.HUD Widget` (`self.Player Character BP`))) (/ _output_get (`self.maxStamina`)))
    (if (<= (`self.currentStamina`) 0.0)
      _
      (else
        (return false))))
  (return true))

(fn `Increase Health`
  (params (AddedHealth :type "Float (double-precision)"))
  (set `self.currentHealth` (+ (`self.currentHealth`) AddedHealth))
  (if (> (`self.currentHealth`) (`self.maxHealth`))
    (bind _output_get (set `self.currentHealth` (`self.maxHealth`)))
    (`ProgressBar.SetPercent` (`/Game/UI/WBP_HUD.HealthBar` (`/Game/ThirdPerson/Blueprints/BP_ThirdPersonCharacter.HUD Widget` (`self.Player Character BP`))) (/ _output_get (`self.maxHealth`)))))

(fn `Increase Max Health`
  (params (`Health Increment` :type "Float (double-precision)"))
  (bind _output_get (set `self.maxHealth` (+ (`self.maxHealth`) `Health Increment`)))
  (bind _output_get_2 (set `self.currentHealth` _output_get))
  (`ProgressBar.SetPercent` (`/Game/UI/WBP_HUD.HealthBar` (`/Game/ThirdPerson/Blueprints/BP_ThirdPersonCharacter.HUD Widget` (`self.Player Character BP`))) (/ _output_get_2 (`self.maxHealth`))))

(fn `Increase Max Stamina`
  (params (AddStamina :type "Float (double-precision)"))
  (bind _output_get (set `self.maxStamina` 0.0))
  (bind _output_get_2 (set `self.currentStamina` _output_get))
  (`ProgressBar.SetPercent` (`/Game/UI/WBP_HUD.StaminaBar` (`/Game/ThirdPerson/Blueprints/BP_ThirdPersonCharacter.HUD Widget` (`self.Player Character BP`))) (/ _output_get_2 (`self.maxStamina`))))

(fn `Increase Stamina`
  (params (AddedStamina :type "Float (double-precision)"))
  (set `self.currentStamina` (+ (`self.currentStamina`) AddedStamina))
  (if (> (`self.currentStamina`) (`self.maxStamina`))
    (bind _output_get (set `self.currentStamina` (`self.maxStamina`))))
  (`ProgressBar.SetPercent` (`/Game/UI/WBP_HUD.StaminaBar` (`/Game/ThirdPerson/Blueprints/BP_ThirdPersonCharacter.HUD Widget` (`self.Player Character BP`))) (/ _output_get (`self.maxStamina`))))

(fn `IncreaseLevel`
  (set `self.level` (+ (`self.level`) 1))
  (set `self.maxXP` (+ (`self.maxXP`) 10.0))
  (set `self.currentXP` 0.0)
  (`TextBlock.SetText` (`/Game/UI/WBP_HUD.LevelText` (`/Game/ThirdPerson/Blueprints/BP_ThirdPersonCharacter.HUD Widget` (`self.Player Character BP`))) (`KismetTextLibrary.Conv_IntToText` (`self.level`)))
  (`GameplayStatics.PlaySound2D` "/Game/Audio/UI/Level_Up.Level_Up" 1.0 1.0 0.0 null null)
  (`GameplayStatics.PlaySound2D` "/Game/Audio/UI/Level_up_2.Level_up_2" 1.0 1.0 0.0 null null))

(fn `IncreaseXP`
  (params (`XP Gained` :type "Float (double-precision)"))
  (set `self.currentXP` (+ (`self.currentXP`) `XP Gained`))
  (if (>= (`self.currentXP`) (`self.maxXP`))
    (`self.IncreaseLevel`))
  (`ProgressBar.SetPercent` (`/Game/UI/WBP_HUD.XPBar` (`/Game/ThirdPerson/Blueprints/BP_ThirdPersonCharacter.HUD Widget` (`self.Player Character BP`))) (/ (`self.currentXP`) (`self.maxXP`)))
  (`TextBlock.SetText` (`/Game/UI/WBP_HUD.XPText` (`/Game/ThirdPerson/Blueprints/BP_ThirdPersonCharacter.HUD Widget` (`self.Player Character BP`))) (`|FormatText` "{currentXP} / {maxXP}" (`self.currentXP`) (`self.maxXP`))))